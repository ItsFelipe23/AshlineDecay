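; BP_Centrifuge is a lab centrifuge prop configured in the construction script, with no runtime logic.
; The construction script rotates the cover around its roll axis by the negated CoverAngle.
; It then adds NumberOfTubes instances to the Tubes instanced mesh, placing each at the component-space transform of the Centrifuge socket named after its index.
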(fn `UserConstructionScript`
  (bind (_returnvalue_location _returnvalue_rotation) (`KismetMathLibrary.BreakTransform` (`SceneComponent.GetSocketTransform` (`self.Centrifuge`) (`KismetStringLibrary.Conv_StringToName` (`KismetStringLibrary.Conv_IntToString` (`self.TubesPlaced`))) "RTS_Component")))
  ;[1 1 1] Cover Movement
  (`SceneComponent.K2_AddLocalRotation` (`self.CentrifugeCover`) (`KismetMathLibrary.MakeRotator` (* (`KismetMathLibrary.Conv_IntToDouble` (`self.CoverAngle`)) -1.0)) false false)
  ;[1 1 1] Adding Tubes
  (for _index (range 1 (+ (`self.NumberOfTubes`) 1))
    (set `self.TubesPlaced` _index)
    (`InstancedStaticMeshComponent.AddInstance` (`self.Tubes`) (`KismetMathLibrary.MakeTransform` _returnvalue_location _returnvalue_rotation) false)))