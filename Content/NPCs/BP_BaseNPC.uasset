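; Base NPC Blueprint that shows an animated interact prompt with the NPC's name and opens that NPC's screen in the player HUD.
; Interact stores the player in SNPCStruct, switches the HUD widget switcher to the NPC's index and hides the prompt.
; If the struct requires a cursor, it also enables game-and-UI input and disables character movement.
; It then calls Functionality, an empty event apparently meant as a child-class hook.
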(event `TogglePlayer`
  (`self.TogglePlayerUI`)
  (`self.Functionality`))

(event `/Game/FirstPerson/Blueprints/Interfaces/BPI_Masters.Interact`
  (params (InteractingPlayer :type "/Game/FirstPerson/Blueprints/BP_BaseFirstPersonCharacter Object Reference"))
  (setmembers `/Game/NPCs/S_NPCStruct` :`StructRef` (`self.S_NPCStruct`) :`PlayerCharacter` InteractingPlayer)
  (`self.TogglePlayer`))

(event `Functionality`)

(event `/Game/FirstPerson/Blueprints/Interfaces/BPI_Masters.ShowPickupUI`
  (bind _aswbp_interact (cast `/Game/UI/WBP_Interact` (`WidgetComponent.GetUserWidgetObject` (`self.InteractWidget`))))
  (bind _structout (setmembers `/Game/NPCs/S_NPCStruct` :`StructRef` (`self.S_NPCStruct`) :`InteractWidget` _aswbp_interact))
  (bind ((`InteractWidget_2_C37E2273455B4082E756B6A3E0CE7A2E` _interactwidget)) (break `/Game/NPCs/S_NPCStruct` _structout))
  (`UserWidget.PlayAnimation` _interactwidget (`/Game/UI/WBP_Interact.PopUp` _interactwidget) 0.0 1 "Forward" 1.5 false)
  (`TextBlock.SetText` (`/Game/UI/WBP_Interact.InteractText` _interactwidget) (`|FormatText` "Press \"E\" to interact with {NPC Name}" (`.NPCName_5_1696153F4C9AB8987E47B281BDE5BAD8` (break `/Game/NPCs/S_NPCStruct` (`self.S_NPCStruct`))))))

(event `/Game/FirstPerson/Blueprints/Interfaces/BPI_Masters.HidePickupUI`
  (`self.HidePrompt`))

(event `HidePrompt`
  (bind ((`InteractWidget_2_C37E2273455B4082E756B6A3E0CE7A2E` _interactwidget)) (break `/Game/NPCs/S_NPCStruct` (`self.S_NPCStruct`)))
  (`/Engine/EditorBlueprintResources/StandardMacros.IsValid` _interactwidget
    (:`Is Valid`
      (`UserWidget.PlayAnimation` _interactwidget (`/Game/UI/WBP_Interact.PopOut` _interactwidget) 0.0 1 "Forward" 1.0 false))))

(fn `TogglePlayerUI`
  (bind _returnvalue (`GameplayStatics.GetPlayerController` 0))
  (bind ((`PlayerCharacter_8_AAE05EE6465EBCF0CC4F33B90ADC4AE2` _playercharacter) (`WidgetIndex_11_462735FA4307A04FA2D9F89098A0BAA0` _widgetindex)) (break `/Game/NPCs/S_NPCStruct` (`self.S_NPCStruct`)))
  (`WidgetSwitcher.SetActiveWidgetIndex` (`/Game/UI/WBP_PlayerHUD.WidgetSwitcher` (`.WBP_PlayerHUD_36_345C8BBE44AD4EDCA59D5696E8C7C791` (break `/Game/FirstPerson/Blueprints/S_PlayerStruct` (`/Game/FirstPerson/Blueprints/BP_BaseFirstPersonCharacter.S_PlayerStruct` _playercharacter)))) _widgetindex)
  (`self.HidePrompt`)
  (if (`.NeedsCursorOnInteract?_13_254FAF7C45287D41824CD3A6500084D7` (break `/Game/NPCs/S_NPCStruct` (`self.S_NPCStruct`)))
    (set `PlayerController.bShowMouseCursor` true _returnvalue)
    (`WidgetBlueprintLibrary.SetInputMode_GameAndUIEx` _returnvalue null)
    (`CharacterMovementComponent.SetMovementMode` (`Character.CharacterMovement` (`.PlayerCharacter_8_AAE05EE6465EBCF0CC4F33B90ADC4AE2` (break `/Game/NPCs/S_NPCStruct` (`self.S_NPCStruct`)))) "MOVE_None" 0)))

(fn `UserConstructionScript`)