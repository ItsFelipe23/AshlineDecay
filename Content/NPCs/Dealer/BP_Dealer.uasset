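; BP_Dealer is a dealer NPC that puts the player into a roulette game when its Functionality event runs.
; The event reveals the Roulette actor's widget, switches the view target to that actor, shows the cursor and sets Game and UI input.
; It disables player movement via movement mode None, then initialises the WBP_RoulettePanel with the player character and the HUD's roulette money display.
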(event `self.ReceiveBeginPlay`
  (`parent.ReceiveBeginPlay`))

(event `self.Functionality`
  (bind _returnvalue (`GameplayStatics.GetPlayerController` 0))
  (bind ((`PlayerCharacter_8_AAE05EE6465EBCF0CC4F33B90ADC4AE2` _playercharacter)) (break `/Game/NPCs/S_NPCStruct` (`self.S_NPCStruct`)))
  (`SceneComponent.SetVisibility` (`/Game/Roulette/BP_Roulette.Widget` (`self.Roulette`)) true false)
  (`PlayerController.SetViewTargetWithBlend` _returnvalue (`self.Roulette`) 0.0 "VTBlend_Linear" 0.0 false)
  (set `PlayerController.bShowMouseCursor` true _returnvalue)
  (`WidgetBlueprintLibrary.SetInputMode_GameAndUIEx` _returnvalue null)
  (`CharacterMovementComponent.SetMovementMode` (`Character.CharacterMovement` (`.PlayerCharacter_8_AAE05EE6465EBCF0CC4F33B90ADC4AE2` (break `/Game/NPCs/S_NPCStruct` (`self.S_NPCStruct`)))) "MOVE_None" 0)
  (bind _aswbp_roulette_panel (cast `/Game/UI/GamblingUI/WBP_RoulettePanel` (`WidgetComponent.GetUserWidgetObject` (`/Game/Roulette/BP_Roulette.Widget` (`self.Roulette`)))))
  (`/Game/UI/GamblingUI/WBP_RoulettePanel.Initialise` _aswbp_roulette_panel _playercharacter)
  (`/Game/UI/WBP_PlayerHUD.InitialiseRouletteMoney` (`.WBP_PlayerHUD_36_345C8BBE44AD4EDCA59D5696E8C7C791` (break `/Game/FirstPerson/Blueprints/S_PlayerStruct` (`/Game/FirstPerson/Blueprints/BP_BaseFirstPersonCharacter.S_PlayerStruct` _playercharacter)))))

(fn `UserConstructionScript`
  (`parent.UserConstructionScript`))