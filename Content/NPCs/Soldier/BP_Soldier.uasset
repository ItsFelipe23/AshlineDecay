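; BP_Soldier is an NPC that presents the mission panel to the player.
; Its Functionality event switches the first player controller's view target to the soldier and hides the player HUD.
; It then initialises and shows the WBP_MissionPanel held by its Widget component, passing in the player character from its NPC struct.
; Finally it disables pickup UI and calls the game instance's quota money update with the current quota.
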(event `self.Functionality`
  (bind _s_playerstruct (`/Game/FirstPerson/Blueprints/BP_BaseFirstPersonCharacter.S_PlayerStruct` (`.PlayerCharacter_8_AAE05EE6465EBCF0CC4F33B90ADC4AE2` (break `/Game/NPCs/S_NPCStruct` (`self.S_NPCStruct`)))))
  (bind ((`GameInstance_39_775371F041515CBBB4FBFC8376C35215` _gameinstance)) (break `/Game/FirstPerson/Blueprints/S_PlayerStruct` _s_playerstruct))
  (`PlayerController.SetViewTargetWithBlend` (`GameplayStatics.GetPlayerController` 0) self 0.0 "VTBlend_Linear" 0.0 false)
  (`Widget.SetVisibility` (`.WBP_PlayerHUD_36_345C8BBE44AD4EDCA59D5696E8C7C791` (break `/Game/FirstPerson/Blueprints/S_PlayerStruct` (`/Game/FirstPerson/Blueprints/BP_BaseFirstPersonCharacter.S_PlayerStruct` (`.PlayerCharacter_8_AAE05EE6465EBCF0CC4F33B90ADC4AE2` (break `/Game/NPCs/S_NPCStruct` (`self.S_NPCStruct`)))))) "Hidden")
  (bind _aswbp_mission_panel (cast `/Game/UI/Missions/WBP_MissionPanel` (`WidgetComponent.GetUserWidgetObject` (`self.Widget`))))
  (`/Game/UI/Missions/WBP_MissionPanel.Initialise` _aswbp_mission_panel (`.PlayerCharacter_8_AAE05EE6465EBCF0CC4F33B90ADC4AE2` (break `/Game/NPCs/S_NPCStruct` (`self.S_NPCStruct`))))
  (`Widget.SetVisibility` _aswbp_mission_panel "Visible")
  (setmembers `/Game/FirstPerson/Blueprints/S_PlayerStruct` :`StructRef` _s_playerstruct :`bCanShowPickupUI` false)
  (`/Game/FirstPerson/Blueprints/BP_ExtractionInstance.E_UpdateQuotaMoney` _gameinstance (`.CurrentQuota_35_D02A22664E7DC8B3C5F638B32BC25508` (break `/Game/FirstPerson/Blueprints/S_GameInstanceStruct` (`/Game/FirstPerson/Blueprints/BP_ExtractionInstance.S_GameInstanceStruct` _gameinstance)))))

(fn `UserConstructionScript`
  (`parent.UserConstructionScript`))