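; BP_Vendor is an NPC vendor that connects the player to the shop UI.
; On BeginPlay it gathers six ItemPlace references into its Basket array.
; Its Functionality event reaches the shop widget through the player character's HUD and initialises it with that player and itself as the vendor.
; The construction script only calls the parent's.
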(event `self.ReceiveBeginPlay`
  (set `self.Basket` (`|MakeArray` (`self.Item Place`) (`self.Item Place1`) (`self.Item Place2`) (`self.Item Place3`) (`self.Item Place4`) (`self.Item Place5`))))

(event `self.Functionality`
  (`/Game/UI/ShopUI/WBP_ShopMenu.Initialise` (`/Game/UI/WBP_PlayerHUD.WBP_ShopUIHUD` (`.WBP_PlayerHUD_36_345C8BBE44AD4EDCA59D5696E8C7C791` (break `/Game/FirstPerson/Blueprints/S_PlayerStruct` (`/Game/FirstPerson/Blueprints/BP_BaseFirstPersonCharacter.S_PlayerStruct` (`.PlayerCharacter_8_AAE05EE6465EBCF0CC4F33B90ADC4AE2` (break `/Game/NPCs/S_NPCStruct` (`self.S_NPCStruct`))))))) (`.PlayerCharacter_8_AAE05EE6465EBCF0CC4F33B90ADC4AE2` (break `/Game/NPCs/S_NPCStruct` (`self.S_NPCStruct`))) self))

(fn `UserConstructionScript`
  (`parent.UserConstructionScript`))