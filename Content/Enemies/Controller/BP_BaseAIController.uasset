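; Base enemy AI controller that runs a behavior tree on BeginPlay and feeds perception updates into its blackboard.
; Sight sets TargetActor to the player while seen, clearing it on loss and requesting a one-second movement prediction.
; Hearing stimuli write TargetLocation.
; The prediction handler writes LastKnownLocation, but compares the stimulus sense against AISenseConfig_Prediction, the config class, rather than a sense class.
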(event `self.ReceiveBeginPlay`
  ;[1 1 1] Runs BT
  (`self.RunBehaviorTree` (`self.BTAsset`)))

(event `self.AIPerception.OnTargetPerceptionUpdated`
  (params (Actor :type "Actor Object Reference") (Stimulus :type "AIStimulus Structure"))
  (`self.HandleSightSense` Actor Stimulus)
  (`self.HandleSoundSense` Stimulus)
  (`self.HandlePredictionSense` Stimulus))

(fn `HandlePredictionSense`
  (params (Stimulus :type "AIStimulus Structure"))
  (bind (_stimulus_age _stimulus_expirationage _stimulus_strength _stimulus_stimuluslocation) (break `AIStimulus` (`local.Stimulus`)))
  (bind _returnvalue (`AIPerceptionSystem.GetSenseClassForStimulus` Stimulus))
  (if (== _returnvalue "/Script/AIModule.AISenseConfig_Prediction")
    (`BlackboardComponent.SetValueAsVector` (`AIBlueprintHelperLibrary.GetBlackboard` null) "LastKnownLocation" _stimulus_stimuluslocation)))

(fn `HandleSightSense`
  (params (Actor :type "Actor Object Reference") (Stimulus :type "AIStimulus Structure"))
  (bind (_stimulus_age _stimulus_expirationage _stimulus_strength _stimulus_stimuluslocation _stimulus_receiverlocation _stimulus_tag _stimulus_bsuccessfullysensed) (break `AIStimulus` (`local.Stimulus`)))
  (bind _returnvalue (`AIPerceptionSystem.GetSenseClassForStimulus` Stimulus))
  (if (== _returnvalue "/Script/AIModule.AISense_Sight")
    (if (`self.ActorHasTag` (`local.Actor`) "Player")
      (`BlackboardComponent.SetValueAsObject` (`AIBlueprintHelperLibrary.GetBlackboard` null) "TargetActor" (`KismetMathLibrary.SelectObject` (`GameplayStatics.GetPlayerCharacter` 0) null _stimulus_bsuccessfullysensed))
      (if (not _stimulus_bsuccessfullysensed)
        (`AISense_Prediction.RequestPawnPredictionEvent` (`self.K2_GetPawn`) (`GameplayStatics.GetPlayerCharacter` 0) 1.0))
      (else
        (return)))
    (else
      (return))))

(fn `HandleSoundSense`
  (params (Stimulus :type "AIStimulus Structure"))
  (bind (_stimulus_age _stimulus_expirationage _stimulus_strength _stimulus_stimuluslocation) (break `AIStimulus` (`local.Stimulus`)))
  (bind _returnvalue (`AIPerceptionSystem.GetSenseClassForStimulus` Stimulus))
  (if (== _returnvalue "/Script/AIModule.AISense_Hearing")
    (`BlackboardComponent.SetValueAsVector` (`AIBlueprintHelperLibrary.GetBlackboard` null) "TargetLocation" _stimulus_stimuluslocation)))

(fn `UserConstructionScript`)