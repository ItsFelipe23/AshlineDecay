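; BP_MasterRoom is a procedural room Blueprint, apparently meant to populate rooms with stibnite pickups and enemies.
; BeginPlay, SpawnRandomActors and the construction script are empty, so the graph currently does nothing.
; Disconnected fragments would roll a stibnite quota, spawn BP_Stibnite at floor spawn points until it is met, and spawn BP_BaseEnemy, storing the latest of each.
; None of these fragments, including a two-way random branch, ever runs.
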(event `self.ReceiveBeginPlay`)

(event `SpawnRandomActors`)

(fn `UserConstructionScript`)