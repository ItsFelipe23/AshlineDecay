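; Interactable door that players swing open and closed, with sound effects and a prompt.
; Interact, ignored while moving, flip-flops the RotateDoor timeline between play and reverse, lerping the mesh's relative rotation from its BeginPlay value to that plus the TargetLoc offset.
; A WBP_Interact widget pops up with open or close text based on IsOpen and pops out when hidden.
; SpawnPurchasedItem is a stub returning false.
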(event `self.ReceiveBeginPlay`
  (`parent.ReceiveBeginPlay`)
  (set `self.StartLoc` (`SceneComponent.RelativeRotation` (`self.Door`))))

(event `/Game/FirstPerson/Blueprints/Interfaces/BPI_Masters.Interact`
  (params (InteractingPlayer :type "/Game/FirstPerson/Blueprints/PlayerCharacter/BP_BaseFirstPersonCharacter Object Reference"))
  (bind _startloc (`self.StartLoc`))
  (set `self.PlayerCharacter` InteractingPlayer)
  (if (not (`self.IsMoving?`))
    (set `self.IsMoving?` true)
    (bind _isa (`/Engine/EditorBlueprintResources/StandardMacros.FlipFlop`)
      (:`A`
        (set `self.isOpen?` _isa)
        (`/Game/FirstPerson/Blueprints/Components/BPC_SFX.PlaySFX` (`self.BPC_SFX`) "/Game/SFX/Doors/SW_DoorOpen.SW_DoorOpen")
        (bind (_direction _moveprogress) (`Timeline|RotateDoor` :!label _label)
          (:`Update`
            (`SceneComponent.K2_SetRelativeRotation` (`self.Door`) (`KismetMathLibrary.RLerp` _startloc (`KismetMathLibrary.ComposeRotators` _startloc (`self.TargetLoc`)) _moveprogress) false false))
          (:`Finished`
            (set `self.IsMoving?` false))))
      (:`B`
        (set `self.isOpen?` _isa)
        (`/Game/FirstPerson/Blueprints/Components/BPC_SFX.PlaySFX` (`self.BPC_SFX`) "/Game/SFX/Doors/SW_DoorClose.SW_DoorClose")
        (goto _label :!via `Reverse`)))))

(event `/Game/FirstPerson/Blueprints/Interfaces/BPI_Masters.ShowPickupUI`
  (bind _aswbp_interact (cast `/Game/UI/WBP_Interact` (`WidgetComponent.GetUserWidgetObject` (`self.Widget`))))
  (bind _output_get (set `self.WBP_Interact` _aswbp_interact))
  (`UserWidget.PlayAnimation` _output_get (`/Game/UI/WBP_Interact.PopUp` _output_get) 0.0 1 "Forward" 1.5 false)
  (if (`self.isOpen?`)
    (`TextBlock.SetText` (`/Game/UI/WBP_Interact.InteractText` _output_get) (`|FormatText` "Press \"E\" to close the door."))
    (else
      (`TextBlock.SetText` (`/Game/UI/WBP_Interact.InteractText` _output_get) (`|FormatText` "Press \"E\" to open the door.")))))

(event `/Game/FirstPerson/Blueprints/Interfaces/BPI_Masters.HidePickupUI`
  (`self.HidePrompt`))

(event `HidePrompt`
  (bind _wbp_interact (`self.WBP_Interact`)
    (:`then`
      (`UserWidget.PlayAnimation` _wbp_interact (`/Game/UI/WBP_Interact.PopOut` _wbp_interact) 0.0 1 "Forward" 1.0 false))
    (:`else`)))

(fn `SpawnPurchasedItem`
  (params (ItemToSpawn :type "/Game/Perks/BP_BaseConsumable Class Reference"))
  (returns (CanSpawn :type Boolean))
  (return false))

(fn `UserConstructionScript`
  (`parent.UserConstructionScript`))