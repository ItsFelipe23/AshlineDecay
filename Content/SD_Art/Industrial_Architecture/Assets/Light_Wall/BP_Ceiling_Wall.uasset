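; BP_Ceiling_Wall is a configurable light fixture pairing a rect light with an emissive static mesh.
; The construction script applies mobility, creates a dynamic material, and sets light properties with matching emissive intensity and temperature-tinted color, or zeroes intensity when off.
; When flickering is enabled on a non-static light, Tick drives light and emissive intensity together with time-based Perlin noise, without checking LightOn.
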(event `self.ReceiveTick`
  (params (DeltaSeconds :type "Float (single-precision)"))
  (bind _returnvalue (`KismetMathLibrary.Lerp` (`self.Min Intensity`) (`self.Intensity`) (/ (+ (`KismetMathLibrary.PerlinNoise1D` (* (`KismetSystemLibrary.GetGameTimeInSeconds`) (`self.Speed`))) 1.0) 2.0)))
  (if (and (`self.Flickering`) (!= (`self.Light Mobility`) 0))
    (`LightComponent.SetIntensity` (`self.RectLight`) _returnvalue)
    (`MeshComponent.SetScalarParameterValueOnMaterials` (`self.StaticMesh`) "Emissive_Intensity" (* _returnvalue (`self.Emissive Multi`)))))

(fn `UserConstructionScript`
  (locals (`Dynamic Mat Inst` :type "MaterialInstanceDynamic Object Reference") (`Temp Color` :type "LinearColor Structure"))
  (bind _returnvalue (`PrimitiveComponent.CreateDynamicMaterialInstance` (`self.StaticMesh`) 0 "/Game/SD_Art/Industrial_Architecture/Assets/Light_Wall/MI_Light_Wall.MI_Light_Wall" "None"))
  (set `local.Dynamic Mat Inst` _returnvalue)
  (`SceneComponent.SetMobility` (`self.RectLight`) (`self.Light Mobility`))
  (if (`self.Light On`)
    (`|ExecutionSequence`
      (:`then_0`
        (`LightComponent.SetIntensity` (`self.RectLight`) (`self.Intensity`))
        (`LightComponent.SetLightColor` (`self.RectLight`) (`self.Light Color`) true)
        (`LocalLightComponent.SetAttenuationRadius` (`self.RectLight`) (`self.Radius`))
        (`LightComponent.SetUseTemperature` (`self.RectLight`) (`self.Use Temperature`))
        (`LightComponent.SetTemperature` (`self.RectLight`) (`self.Temperature`))
        (`LightComponent.SetIndirectLightingIntensity` (`self.RectLight`) (`self.Indirect Intensity`))
        (`LightComponent.SetVolumetricScatteringIntensity` (`self.RectLight`) (`self.Volumetric Intensity`)))
      (:`then_1`
        (`MeshComponent.SetScalarParameterValueOnMaterials` (`self.StaticMesh`) "Emissive_Intensity" (* (`self.Intensity`) (`self.Emissive Multi`)))
        (`KismetMathLibrary.LinearColor_SetTemperature` (`local.Temp Color`) (`self.Temperature`))
        (`MeshComponent.SetVectorParameterValueOnMaterials` (`self.StaticMesh`) "Emissive_Color" (`KismetMathLibrary.Conv_LinearColorToVector` (* (`local.Temp Color`) (`self.Light Color`))))))
    (else
      (`LightComponent.SetIntensity` (`self.RectLight`) 0.0)
      (`MeshComponent.SetScalarParameterValueOnMaterials` (`self.StaticMesh`) "Emissive_Intensity" 0.0))))