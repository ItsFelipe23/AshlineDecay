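; Configurable industrial fluorescent lamp prop with a main spot light, fog rect light, two side rect lights and an emissive mesh.
; The construction script applies mobility, intensity, color, temperature and radius settings, deriving secondary intensities and emissive glow from one Intensity, or zeroes them when LightOn is false.
; When Flickering is enabled and main light mobility isn't Static, Tick drives lights and emissive with Perlin noise, without checking LightOn.
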(event `self.ReceiveTick`
  (params (DeltaSeconds :type "Float (single-precision)"))
  (bind _returnvalue (`KismetMathLibrary.Lerp` (`self.Min Intensity`) (`self.Intensity`) (/ (+ (`KismetMathLibrary.PerlinNoise1D` (* (`KismetSystemLibrary.GetGameTimeInSeconds`) (`self.Speed`))) 1.0) 2.0)))
  (bind _returnvalue_2 (* _returnvalue 0.035))
  (if (and (`self.Flickering`) (!= (`self.Light Mobility Main`) 0))
    (`LightComponent.SetIntensity` (`self.SpotLight_Main`) _returnvalue)
    (`LightComponent.SetIntensity` (`self.RectLight_Fog`) (* _returnvalue 0.001))
    (`LightComponent.SetIntensity` (`self.RectLight_Up`) _returnvalue_2)
    (`LightComponent.SetIntensity` (`self.RectLight_Down`) _returnvalue_2)
    (`MeshComponent.SetScalarParameterValueOnMaterials` (`self.SM_Light_Wall_02_`) "Emissive_Intensity" (* _returnvalue (`self.Emissive Multi`)))))

(fn `UserConstructionScript`
  (locals (`Dynamic Mat Inst` :type "MaterialInstanceDynamic Object Reference") (`Temp Color` :type "LinearColor Structure"))
  (bind _returnvalue (* (`self.Intensity`) 0.035))
  (bind _returnvalue_2 (`PrimitiveComponent.CreateDynamicMaterialInstance` (`self.SM_Light_Wall_02_`) 0 "/Game/SD_Art/Industrial_Architecture/Assets/Light_Wall_Big/MI_Light_Wall_Big.MI_Light_Wall_Big" "None"))
  (set `local.Dynamic Mat Inst` _returnvalue_2)
  (`SceneComponent.SetMobility` (`self.SpotLight_Main`) (`self.Light Mobility Main`))
  (`SceneComponent.SetMobility` (`self.RectLight_Up`) (`self.Light Mobility Side`))
  (`SceneComponent.SetMobility` (`self.RectLight_Down`) (`self.Light Mobility Side`))
  (if (`self.Light On`)
    (`|ExecutionSequence`
      (:`then_0`
        (`LightComponent.SetIntensity` (`self.SpotLight_Main`) (`self.Intensity`))
        (`LightComponent.SetLightColor` (`self.SpotLight_Main`) (`self.Light Color`) true)
        (`LocalLightComponent.SetAttenuationRadius` (`self.SpotLight_Main`) (`self.Radius`))
        (`LightComponent.SetUseTemperature` (`self.SpotLight_Main`) (`self.Use Temperature`))
        (`LightComponent.SetTemperature` (`self.SpotLight_Main`) (`self.Temperature`))
        (`LightComponent.SetIndirectLightingIntensity` (`self.SpotLight_Main`) (`self.Indirect Intensity`)))
      (:`then_1`
        (`LightComponent.SetIntensity` (`self.RectLight_Fog`) (* (`self.Intensity`) 0.001))
        (`LightComponent.SetLightColor` (`self.RectLight_Fog`) (`self.Light Color`) true)
        (`LocalLightComponent.SetAttenuationRadius` (`self.RectLight_Fog`) (`self.Fog Radius`))
        (`LightComponent.SetUseTemperature` (`self.RectLight_Fog`) (`self.Use Temperature`))
        (`LightComponent.SetTemperature` (`self.RectLight_Fog`) (`self.Temperature`))
        (`LightComponent.SetVolumetricScatteringIntensity` (`self.RectLight_Fog`) (`self.Volumetric Intensity`)))
      (:`then_2`
        (`LightComponent.SetIntensity` (`self.RectLight_Up`) _returnvalue)
        (`LightComponent.SetIntensity` (`self.RectLight_Down`) _returnvalue)
        (`LightComponent.SetLightColor` (`self.RectLight_Up`) (`self.Light Color`) true)
        (`LightComponent.SetLightColor` (`self.RectLight_Down`) (`self.Light Color`) true)
        (`LocalLightComponent.SetAttenuationRadius` (`self.RectLight_Up`) (`self.Side Light Radius`))
        (`LocalLightComponent.SetAttenuationRadius` (`self.RectLight_Down`) (`self.Side Light Radius`))
        (`LightComponent.SetUseTemperature` (`self.RectLight_Up`) (`self.Use Temperature`))
        (`LightComponent.SetUseTemperature` (`self.RectLight_Down`) (`self.Use Temperature`))
        (`LightComponent.SetTemperature` (`self.RectLight_Up`) (`self.Temperature`))
        (`LightComponent.SetTemperature` (`self.RectLight_Down`) (`self.Temperature`)))
      (:`then_3`
        (`MeshComponent.SetScalarParameterValueOnMaterials` (`self.SM_Light_Wall_02_`) "Emissive_Intensity" (* (`self.Intensity`) (`self.Emissive Multi`)))
        (`KismetMathLibrary.LinearColor_SetTemperature` (`local.Temp Color`) (`self.Temperature`))
        (`MeshComponent.SetVectorParameterValueOnMaterials` (`self.SM_Light_Wall_02_`) "Emissive_Color" (`KismetMathLibrary.Conv_LinearColorToVector` (* (`local.Temp Color`) (`self.Light Color`))))))
    (else
      (`LightComponent.SetIntensity` (`self.SpotLight_Main`) 0.0)
      (`LightComponent.SetIntensity` (`self.RectLight_Fog`) 0.0)
      (`LightComponent.SetIntensity` (`self.RectLight_Up`) 0.0)
      (`LightComponent.SetIntensity` (`self.RectLight_Down`) 0.0)
      (`MeshComponent.SetScalarParameterValueOnMaterials` (`self.SM_Light_Wall_02_`) "Emissive_Intensity" 0.0))))