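; Alarm lamp actor pairing a point light with an emissive bunker wall-light mesh, with optional flashing.
; Construction script applies the exposed light settings and matches emissive intensity and temperature-tinted color, or zeroes both light and glow when LightOn is off.
; Tick reapplies the settings without checking LightOn; LightFlashing scales light and glow by a game-time sine.
; Tick also calls CreateDynamicMaterialInstance every frame rather than using the stored DynamicMatInst.
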(event `self.ReceiveTick`
  (params (DeltaSeconds :type "Float (single-precision)"))
  (bind _sm_light_small_bunker_wall_01_ (`self.SM_Light_Small_Bunker_Wall_01_`))
  (bind _intensity (`self.Intensity`))
  (bind _pointlight (`self.PointLight`))
  (bind _returnvalue (`PrimitiveComponent.GetMaterial` _sm_light_small_bunker_wall_01_ 0))
  (bind _returnvalue_2 (`KismetMathLibrary.Lerp` 0.0 _intensity (`KismetMathLibrary.Sin` (* (`KismetSystemLibrary.GetGameTimeInSeconds`) (`self.Speed`)))))
  (`|ExecutionSequence`
    (:`then_0`
      (`LightComponent.SetIntensity` (`self.PointLight`) (`self.Intensity`))
      (`LightComponent.SetLightColor` (`self.PointLight`) (`self.Light Color`) true)
      (`LocalLightComponent.SetAttenuationRadius` (`self.PointLight`) (`self.Radius`))
      (`LightComponent.SetUseTemperature` (`self.PointLight`) (`self.Use Temperature`))
      (`LightComponent.SetTemperature` (`self.PointLight`) (`self.Temperature`))
      (`LightComponent.SetIndirectLightingIntensity` (`self.PointLight`) (`self.Indirect Intensity`))
      (`LightComponent.SetVolumetricScatteringIntensity` (`self.PointLight`) (`self.Volumetric Intensity`)))
    (:`then_1`
      (`MeshComponent.SetScalarParameterValueOnMaterials` (`self.SM_Light_Small_Bunker_Wall_01_`) "Emissive_Intensity" (* (`self.Intensity`) (`self.Emissive Multi`)))
      (`KismetMathLibrary.LinearColor_SetTemperature` (`self.In Out Color`) (`self.Temperature`))
      (`MeshComponent.SetVectorParameterValueOnMaterials` (`self.SM_Light_Small_Bunker_Wall_01_`) "Emissive_Color" (`KismetMathLibrary.Conv_LinearColorToVector` (* (`self.In Out Color`) (`self.Light Color`)))))
    (:`then_2`
      (if (`self.Light Flashing`)
        (`LightComponent.SetIntensity` _pointlight _returnvalue_2)
        (bind _returnvalue_3 (`PrimitiveComponent.CreateDynamicMaterialInstance` _sm_light_small_bunker_wall_01_ 0 _returnvalue "None"))
        (`MaterialInstanceDynamic.SetScalarParameterValue` _returnvalue_3 "Emissive_Intensity" (* _returnvalue_2 (`self.Emissive Multi`)))
        (else
          (`LightComponent.SetIntensity` _pointlight _intensity)
          (bind _returnvalue_4 (`PrimitiveComponent.CreateDynamicMaterialInstance` _sm_light_small_bunker_wall_01_ 0 _returnvalue "None"))
          (`MaterialInstanceDynamic.SetScalarParameterValue` _returnvalue_4 "Emissive_Intensity" (* _intensity (`self.Emissive Multi`))))))))

(fn `UserConstructionScript`
  (locals (`Dynamic Mat Inst` :type "MaterialInstanceDynamic Object Reference") (`Temp Color` :type "LinearColor Structure"))
  (bind _returnvalue (`PrimitiveComponent.CreateDynamicMaterialInstance` (`self.SM_Light_Small_Bunker_Wall_01_`) 0 "/Game/SD_Art/Industrial_Architecture/Assets/Light_Wall_Bunker_Small/MI_Light_Small_Bunker_Wall.MI_Light_Small_Bunker_Wall" "None"))
  (set `local.Dynamic Mat Inst` _returnvalue)
  (`SceneComponent.SetMobility` (`self.PointLight`) (`self.Light Mobility`))
  (if (`self.Light On`)
    (`|ExecutionSequence`
      (:`then_0`
        (`LightComponent.SetIntensity` (`self.PointLight`) (`self.Intensity`))
        (`LightComponent.SetLightColor` (`self.PointLight`) (`self.Light Color`) true)
        (`LocalLightComponent.SetAttenuationRadius` (`self.PointLight`) (`self.Radius`))
        (`LightComponent.SetUseTemperature` (`self.PointLight`) (`self.Use Temperature`))
        (`LightComponent.SetTemperature` (`self.PointLight`) (`self.Temperature`))
        (`LightComponent.SetIndirectLightingIntensity` (`self.PointLight`) (`self.Indirect Intensity`))
        (`LightComponent.SetVolumetricScatteringIntensity` (`self.PointLight`) (`self.Volumetric Intensity`)))
      (:`then_1`
        (`MeshComponent.SetScalarParameterValueOnMaterials` (`self.SM_Light_Small_Bunker_Wall_01_`) "Emissive_Intensity" (* (`self.Intensity`) (`self.Emissive Multi`)))
        (`KismetMathLibrary.LinearColor_SetTemperature` (`local.Temp Color`) (`self.Temperature`))
        (`MeshComponent.SetVectorParameterValueOnMaterials` (`self.SM_Light_Small_Bunker_Wall_01_`) "Emissive_Color" (`KismetMathLibrary.Conv_LinearColorToVector` (* (`local.Temp Color`) (`self.Light Color`))))))
    (else
      (`LightComponent.SetIntensity` (`self.PointLight`) 0.0)
      (`MeshComponent.SetScalarParameterValueOnMaterials` (`self.SM_Light_Small_Bunker_Wall_01_`) "Emissive_Intensity" 0.0))))