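; A camera and speaker system prop Blueprint from the industrial architecture art set, with two adjustable speaker meshes.
; The construction script places each speaker using exposed height and yaw rotation variables and toggles each one's visibility with its own flag.
; All event graph nodes are disabled stubs, so the asset has no runtime logic.
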(fn `UserConstructionScript`
  (bind _sm_speaker_01_ (`self.SM_Speaker_01_`))
  (bind _sm_speaker_02_ (`self.SM_Speaker_02_`))
  (`SceneComponent.K2_SetRelativeTransform` _sm_speaker_01_ (`KismetMathLibrary.MakeTransform` (`KismetMathLibrary.MakeVector` 0.0 0.0 (`self.Speaker_01_Height`)) (`KismetMathLibrary.MakeRotator` 0.0 0.0 (`self.Speaker_01_Rotation`))) false false)
  (`SceneComponent.K2_SetRelativeTransform` _sm_speaker_02_ (`KismetMathLibrary.MakeTransform` (`KismetMathLibrary.MakeVector` 0.0 0.0 (`self.Speaker_02_Height`)) (`KismetMathLibrary.MakeRotator` 0.0 0.0 (`self.Speaker_02_Rotation`))) false false)
  (`SceneComponent.SetVisibility` _sm_speaker_02_ (`self.Speaker_02_Visible`) false)
  (`SceneComponent.SetVisibility` _sm_speaker_01_ (`self.Speaker_01_Visible`) false))