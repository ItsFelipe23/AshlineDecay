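; Construction-script mesh repeater that lays out a row of industrial pipe presets or a custom mesh along a chosen axis.
; Spacing comes from the mesh's local bounds plus an offset, with incremental rotation about that axis per copy.
; AllowVertexPainting spawns separate static mesh components; otherwise one instanced static mesh holds every copy.
; Pipe type selects mesh and material, with an optional color overlay set through material parameters.
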(fn `UserConstructionScript`
  (locals (Pipes_Mesh :type "InstancedStaticMeshComponent Object Reference") (Pipes_Mesh_Static :type "StaticMeshComponent Object Reference"))
  (bind _custom_color_overlay (`self.Custom_Color_Overlay`))
  (bind _use_color_overlay (`self.Use_Color_Overlay`))
  (bind _pipes_mesh (`local.Pipes_Mesh`))
  (bind _pipes_mesh_2 (`local.Pipes_Mesh`))
  (bind _pipes_mesh_3 (`local.Pipes_Mesh`))
  (bind _pipes_mesh_static (`local.Pipes_Mesh_Static`))
  (bind _pipes_mesh_static_2 (`local.Pipes_Mesh_Static`))
  (bind _pipes_mesh_static_3 (`local.Pipes_Mesh_Static`))
  (bind _pipes_mesh_static_4 (`local.Pipes_Mesh_Static`))
  (bind _pipes_mesh_static_5 (`local.Pipes_Mesh_Static`))
  (bind _pipes_mesh_static_6 (`local.Pipes_Mesh_Static`))
  (bind (_min _max) (`StaticMeshComponent.GetLocalBounds` (`local.Pipes_Mesh`)))
  (bind (_min_2 _max_2) (`StaticMeshComponent.GetLocalBounds` (`local.Pipes_Mesh`)))
  (bind (_min_3 _max_3) (`StaticMeshComponent.GetLocalBounds` (`local.Pipes_Mesh_Static`)))
  (bind (_min_4 _max_4) (`StaticMeshComponent.GetLocalBounds` (`local.Pipes_Mesh_Static`)))
  (bind (_min_5 _max_5) (`StaticMeshComponent.GetLocalBounds` (`local.Pipes_Mesh_Static`)))
  (bind (_min_6 _max_6) (`StaticMeshComponent.GetLocalBounds` (`local.Pipes_Mesh`)))
  (if (`self.Allow Vertex Painting`)
    (switch `/Game/SD_Art/Industrial_Architecture/Blueprints/Enumerations/E_Asset_Axis` (`self.Asset_Axis`)
      (:`NewEnumerator3`
        (for _index (range (`self.Amount`))
          (bind _returnvalue (`AddComponent|NODE_AddStaticMeshComponent-0` :`RelativeTransform` (`KismetMathLibrary.MakeTransform` (`KismetMathLibrary.MakeVector` (* (`KismetMathLibrary.Conv_IntToDouble` _index) (`KismetMathLibrary.Conv_IntToDouble` (`KismetMathLibrary.Conv_Int64ToInt` (`KismetMathLibrary.Round64` (+ (`self.Position_Offset`) (- (.x _max_3) (.x _min_3)))))))) (`KismetMathLibrary.MakeRotator` (* (`KismetMathLibrary.Conv_IntToDouble` _index) (`self.Rotation_Amount`))))))
          (set `local.Pipes_Mesh_Static` _returnvalue)
          (switch `/Game/SD_Art/Industrial_Architecture/Blueprints/Enumerations/E_Pipe_Types` (`self.Pipe_Types`) :!label _label
            (:`NewEnumerator3`
              (`StaticMeshComponent.SetStaticMesh` _pipes_mesh_static (`self.Custom_Mesh`))
              (if (`self.Custom Material`)
                (`PrimitiveComponent.SetMaterial` _pipes_mesh_static 0 (`self.Custom_Material`)))
              (if (`self.Use_Color_Overlay`)
                (`MeshComponent.SetVectorParameterValueOnMaterials` _pipes_mesh_static "Albedo_1_ColorOverlay" (`KismetMathLibrary.Conv_LinearColorToVector` (`self.Custom_Color_Overlay`)))
                (`MeshComponent.SetScalarParameterValueOnMaterials` _pipes_mesh_static "Color_Mask_1_Intensity" (`self.Color_Mask_Intensity`))))
            (:`NewEnumerator0`
              (`StaticMeshComponent.SetStaticMesh` _pipes_mesh_static (`self.Pipe_Small_4M`))
              (`PrimitiveComponent.SetMaterial` _pipes_mesh_static_6 0 (`self.Pipes_Small`) :!label _label_2)
              (if _use_color_overlay
                (`MeshComponent.SetVectorParameterValueOnMaterials` _pipes_mesh_static_6 "Albedo_1_ColorOverlay" (`KismetMathLibrary.Conv_LinearColorToVector` _custom_color_overlay))
                (`MeshComponent.SetScalarParameterValueOnMaterials` _pipes_mesh_static_6 "Color_Mask_1_Intensity" (`self.Color_Mask_Intensity`))))
            (:`NewEnumerator1`
              (`StaticMeshComponent.SetStaticMesh` _pipes_mesh_static (`self.Pipe_Small_2M`))
              (goto _label_2))
            (:`NewEnumerator2`
              (`StaticMeshComponent.SetStaticMesh` _pipes_mesh_static (`self.Pipe_Small_1M`))
              (goto _label_2))
            (:`NewEnumerator4`
              (`StaticMeshComponent.SetStaticMesh` _pipes_mesh_static_2 (`self.Pipe_Medium_4M`))
              (`PrimitiveComponent.SetMaterial` _pipes_mesh_static_5 0 (`self.Pipes_Medium`) :!label _label_3)
              (if _use_color_overlay
                (`MeshComponent.SetVectorParameterValueOnMaterials` _pipes_mesh_static_5 "Albedo_1_ColorOverlay" (`KismetMathLibrary.Conv_LinearColorToVector` _custom_color_overlay))
                (`MeshComponent.SetScalarParameterValueOnMaterials` _pipes_mesh_static_5 "Color_Mask_1_Intensity" (`self.Color_Mask_Intensity`))))
            (:`NewEnumerator5`
              (`StaticMeshComponent.SetStaticMesh` _pipes_mesh_static_2 (`self.Pipe_Medium_2M`))
              (goto _label_3))
            (:`NewEnumerator6`
              (`StaticMeshComponent.SetStaticMesh` _pipes_mesh_static_2 (`self.Pipe_Medium_1M`))
              (goto _label_3))
            (:`NewEnumerator7`
              (`StaticMeshComponent.SetStaticMesh` _pipes_mesh_static_3 (`self.Pipe_Large_4M`))
              (`PrimitiveComponent.SetMaterial` _pipes_mesh_static_4 0 (`self.Pipes_Large`) :!label _label_4)
              (if _use_color_overlay
                (`MeshComponent.SetVectorParameterValueOnMaterials` _pipes_mesh_static_4 "Albedo_1_ColorOverlay" (`KismetMathLibrary.Conv_LinearColorToVector` _custom_color_overlay))
                (`MeshComponent.SetScalarParameterValueOnMaterials` _pipes_mesh_static_4 "Color_Mask_1_Intensity" (`self.Color_Mask_Intensity`))))
            (:`NewEnumerator8`
              (`StaticMeshComponent.SetStaticMesh` _pipes_mesh_static_3 (`self.Pipe_Large_2M`))
              (goto _label_4))
            (:`NewEnumerator9`
              (`StaticMeshComponent.SetStaticMesh` _pipes_mesh_static_3 (`self.Pipe_Large_1M`))
              (goto _label_4)))))
      (:`NewEnumerator0`
        (for _index_2 (range (`self.Amount`))
          (bind _returnvalue_2 (`AddComponent|NODE_AddStaticMeshComponent-4` :`RelativeTransform` (`KismetMathLibrary.MakeTransform` (`KismetMathLibrary.MakeVector` 0.0 (* (`KismetMathLibrary.Conv_IntToDouble` _index_2) (`KismetMathLibrary.Conv_IntToDouble` (`KismetMathLibrary.Conv_Int64ToInt` (`KismetMathLibrary.Round64` (+ (`self.Position_Offset`) (- (.y _max_5) (.y _min_5)))))))) (`KismetMathLibrary.MakeRotator` 0.0 (* (`KismetMathLibrary.Conv_IntToDouble` _index_2) (`self.Rotation_Amount`))))))
          (set `local.Pipes_Mesh_Static` _returnvalue_2)
          (goto _label)))
      (:`NewEnumerator1`
        (for _index_3 (range (`self.Amount`))
          (bind _returnvalue_3 (`AddComponent|NODE_AddStaticMeshComponent-5` :`RelativeTransform` (`KismetMathLibrary.MakeTransform` (`KismetMathLibrary.MakeVector` 0.0 0.0 (* (`KismetMathLibrary.Conv_IntToDouble` _index_3) (`KismetMathLibrary.Conv_IntToDouble` (`KismetMathLibrary.Conv_Int64ToInt` (`KismetMathLibrary.Round64` (+ (`self.Position_Offset`) (- (.z _max_4) (.z _min_4)))))))) (`KismetMathLibrary.MakeRotator` 0.0 0.0 (* (`KismetMathLibrary.Conv_IntToDouble` _index_3) (`self.Rotation_Amount`))))))
          (set `local.Pipes_Mesh_Static` _returnvalue_3)
          (goto _label))))
    (else
      (bind _returnvalue_4 (`AddComponent|NODE_AddInstancedStaticMeshComponent-0`))
      (set `local.Pipes_Mesh` _returnvalue_4)
      (switch `/Game/SD_Art/Industrial_Architecture/Blueprints/Enumerations/E_Pipe_Types` (`self.Pipe_Types`)
        (:`NewEnumerator3`
          (`StaticMeshComponent.SetStaticMesh` _pipes_mesh (`self.Custom_Mesh`))
          (if (`self.Custom Material`)
            (`PrimitiveComponent.SetMaterial` _pipes_mesh 0 (`self.Custom_Material`))
            (if (`self.Use_Color_Overlay`) :!label _label_5
              (`MeshComponent.SetVectorParameterValueOnMaterials` _pipes_mesh "Albedo_1_ColorOverlay" (`KismetMathLibrary.Conv_LinearColorToVector` (`self.Custom_Color_Overlay`)))
              (`MeshComponent.SetScalarParameterValueOnMaterials` _pipes_mesh "Color_Mask_1_Intensity" (`self.Color_Mask_Intensity`)))))
        (:`NewEnumerator0`
          (`StaticMeshComponent.SetStaticMesh` _pipes_mesh (`self.Pipe_Small_4M`))
          (`PrimitiveComponent.SetMaterial` (`local.Pipes_Mesh`) 0 (`self.Pipes_Small`) :!label _label_6)
          (goto _label_5))
        (:`NewEnumerator1`
          (`StaticMeshComponent.SetStaticMesh` _pipes_mesh (`self.Pipe_Small_2M`))
          (goto _label_6))
        (:`NewEnumerator2`
          (`StaticMeshComponent.SetStaticMesh` _pipes_mesh (`self.Pipe_Small_1M`))
          (goto _label_6))
        (:`NewEnumerator4`
          (`StaticMeshComponent.SetStaticMesh` _pipes_mesh_2 (`self.Pipe_Medium_4M`))
          (`PrimitiveComponent.SetMaterial` (`local.Pipes_Mesh`) 0 (`self.Pipes_Medium`) :!label _label_7)
          (goto _label_5))
        (:`NewEnumerator5`
          (`StaticMeshComponent.SetStaticMesh` _pipes_mesh_2 (`self.Pipe_Medium_2M`))
          (goto _label_7))
        (:`NewEnumerator6`
          (`StaticMeshComponent.SetStaticMesh` _pipes_mesh_2 (`self.Pipe_Medium_1M`))
          (goto _label_7))
        (:`NewEnumerator7`
          (`StaticMeshComponent.SetStaticMesh` _pipes_mesh_3 (`self.Pipe_Large_4M`))
          (`PrimitiveComponent.SetMaterial` (`local.Pipes_Mesh`) 0 (`self.Pipes_Large`) :!label _label_8)
          (goto _label_5))
        (:`NewEnumerator8`
          (`StaticMeshComponent.SetStaticMesh` _pipes_mesh_3 (`self.Pipe_Large_2M`))
          (goto _label_8))
        (:`NewEnumerator9`
          (`StaticMeshComponent.SetStaticMesh` _pipes_mesh_3 (`self.Pipe_Large_1M`))
          (goto _label_8)))
      (switch `/Game/SD_Art/Industrial_Architecture/Blueprints/Enumerations/E_Asset_Axis` (`self.Asset_Axis`)
        (:`NewEnumerator3`
          (for _index_4 (range (`self.Amount`))
            (`InstancedStaticMeshComponent.AddInstance` (`local.Pipes_Mesh`) (`KismetMathLibrary.MakeTransform` (`KismetMathLibrary.MakeVector` (* (`KismetMathLibrary.Conv_IntToDouble` _index_4) (`KismetMathLibrary.Conv_IntToDouble` (`KismetMathLibrary.Conv_Int64ToInt` (`KismetMathLibrary.Round64` (+ (`self.Position_Offset`) (- (.x _max_6) (.x _min_6)))))))) (`KismetMathLibrary.MakeRotator` (* (`KismetMathLibrary.Conv_IntToDouble` _index_4) (`self.Rotation_Amount`)))) false)))
        (:`NewEnumerator0`
          (for _index_5 (range (`self.Amount`))
            (`InstancedStaticMeshComponent.AddInstance` (`local.Pipes_Mesh`) (`KismetMathLibrary.MakeTransform` (`KismetMathLibrary.MakeVector` 0.0 (* (`KismetMathLibrary.Conv_IntToDouble` _index_5) (`KismetMathLibrary.Conv_IntToDouble` (`KismetMathLibrary.Conv_Int64ToInt` (`KismetMathLibrary.Round64` (+ (`self.Position_Offset`) (- (.y _max) (.y _min)))))))) (`KismetMathLibrary.MakeRotator` 0.0 (* (`KismetMathLibrary.Conv_IntToDouble` _index_5) (`self.Rotation_Amount`)))) false)))
        (:`NewEnumerator1`
          (for _index_6 (range (`self.Amount`))
            (`InstancedStaticMeshComponent.AddInstance` (`local.Pipes_Mesh`) (`KismetMathLibrary.MakeTransform` (`KismetMathLibrary.MakeVector` 0.0 0.0 (* (`KismetMathLibrary.Conv_IntToDouble` _index_6) (`KismetMathLibrary.Conv_IntToDouble` (`KismetMathLibrary.Conv_Int64ToInt` (`KismetMathLibrary.Round64` (+ (`self.Position_Offset`) (- (.z _max_2) (.z _min_2)))))))) (`KismetMathLibrary.MakeRotator` 0.0 0.0 (* (`KismetMathLibrary.Conv_IntToDouble` _index_6) (`self.Rotation_Amount`)))) false)))))))