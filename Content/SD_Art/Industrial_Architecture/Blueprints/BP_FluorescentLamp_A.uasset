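; Fluorescent ceiling lamp prop with a spot light, a rect light for volumetric fog and an emissive fixture mesh.
; TurnOn pushes shared intensity, color and temperature settings to both lights, scaling the fog light far down.
; It also drives the mesh's emissive brightness and temperature-tinted color.
; The construction script is empty; its LightOn toggle, mobility and dynamic-material setup are disconnected and never run.
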(event `TurnOn`
  (set `self.Emissive Multi` 50.0)
  (`|ExecutionSequence`
    (:`then_0`
      (`LightComponent.SetIntensity` (`self.SpotLight_Main`) (`self.Intensity`))
      (`LightComponent.SetLightColor` (`self.SpotLight_Main`) (`self.Light Color`) true)
      (`LocalLightComponent.SetAttenuationRadius` (`self.SpotLight_Main`) (`self.Radius`))
      (`LightComponent.SetUseTemperature` (`self.SpotLight_Main`) (`self.Use Temperature`))
      (`LightComponent.SetTemperature` (`self.SpotLight_Main`) (`self.Temperature`))
      (`LightComponent.SetIndirectLightingIntensity` (`self.SpotLight_Main`) (`self.Indirect Intensity`)))
    (:`then_1`
      (`LightComponent.SetIntensity` (`self.RectLight_Fog`) (* (`self.Intensity`) 0.001))
      (`LightComponent.SetLightColor` (`self.RectLight_Fog`) (`self.Light Color`) true)
      (`LocalLightComponent.SetAttenuationRadius` (`self.RectLight_Fog`) (`self.Fog Radius`))
      (`LightComponent.SetUseTemperature` (`self.RectLight_Fog`) (`self.Use Temperature`))
      (`LightComponent.SetTemperature` (`self.RectLight_Fog`) (`self.Temperature`))
      (`LightComponent.SetVolumetricScatteringIntensity` (`self.RectLight_Fog`) (`self.Volumetric Intensity`)))
    (:`then_2`
      (`MeshComponent.SetScalarParameterValueOnMaterials` (`self.SM_Ceiling_Light_01_`) "Emissive_Intensity" (* (`self.Intensity`) (`self.Emissive Multi`)))
      (`KismetMathLibrary.LinearColor_SetTemperature` (`self.Temp Color`) (`self.Temperature`))
      (`MeshComponent.SetVectorParameterValueOnMaterials` (`self.SM_Ceiling_Light_01_`) "Emissive_Color" (`KismetMathLibrary.Conv_LinearColorToVector` (* (`self.Temp Color`) (`self.Light Color`)))))))

(fn `UserConstructionScript`
  (locals (`Dynamic Mat Inst` :type "MaterialInstanceDynamic Object Reference") (`Temp Color` :type "LinearColor Structure")))