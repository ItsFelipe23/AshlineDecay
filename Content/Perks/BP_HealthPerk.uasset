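; BP_HealthPerk is a perk item that raises the owning character's maximum health to a fixed value when used.
; Its UseItem override calls the parent, then sets MaxHealth on the health component of the character stored in SItemsStruct.
; It copies that maximum into both current and max health in the player attributes struct, then passes both to the character's health-updated call.
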(fn `Use Item`
  (params (PlayerREF :type "/Game/FirstPerson/Blueprints/BP_BaseFirstPersonCharacter Object Reference"))
  (`parent.Use Item` PlayerREF)
  (bind _output_get (set `/Game/FirstPerson/Blueprints/Components/BPC_HealthComponent.MaxHealth` 150.0 (`/Game/FirstPerson/Blueprints/BP_BaseFirstPersonCharacter.BPC_HealthComponent` (`.OwningCharacter_39_92B2FB504539D6CF5DCE6AAE7DB5BE06` (break `/Game/FirstPerson/Blueprints/Items/S_Items` (`self.S_ItemsStruct`))))))
  (bind _structout (setmembers `/Game/FirstPerson/Blueprints/S_PlayerAttributes` :`StructRef` (`/Game/FirstPerson/Blueprints/BP_BaseFirstPersonCharacter.S_PlayerAttributes` (`.OwningCharacter_39_92B2FB504539D6CF5DCE6AAE7DB5BE06` (break `/Game/FirstPerson/Blueprints/Items/S_Items` (`self.S_ItemsStruct`)))) :`CurrentHealth` _output_get :`MaxHealth` _output_get))
  (bind ((`CurrentHealth_4_FE1E194646813E0C90C81281091CC508` _currenthealth) (`MaxHealth_41_BAD91A2C4FD2E3C89646BBA705DFCD60` _maxhealth)) (break `/Game/FirstPerson/Blueprints/S_PlayerAttributes` _structout))
  (`/Game/FirstPerson/Blueprints/BP_BaseFirstPersonCharacter.E_HealthUpdated` (`.OwningCharacter_39_92B2FB504539D6CF5DCE6AAE7DB5BE06` (break `/Game/FirstPerson/Blueprints/Items/S_Items` (`self.S_ItemsStruct`))) _currenthealth _maxhealth))

(fn `UserConstructionScript`
  (`parent.UserConstructionScript`))