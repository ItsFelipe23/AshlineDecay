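; BP_MutationEndurancePerk is a usable perk item that changes how radiation zones are tuned when used.
; Its Use Item override runs the parent logic, then finds a single BP_RadiationZone via GetActorOfClass.
; It zeroes that zone's low and mid radiation values and sets the high value to a small fixed amount, leaving any other zone instances untouched.
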(fn `Use Item`
  (params (PlayerREF :type "/Game/FirstPerson/Blueprints/BP_BaseFirstPersonCharacter Object Reference"))
  (bind _raditaionzoneref (`self.RaditaionZoneREF`))
  (`parent.Use Item` PlayerREF)
  (bind _returnvalue (`GameplayStatics.GetActorOfClass` "/Game/Radiation/BP_RadiationZone.BP_RadiationZone_C"))
  (bind _output_get (set `self.RaditaionZoneREF` _returnvalue))
  (set `/Game/Radiation/BP_RadiationZone.LowRadiation` 0.0 _output_get)
  (set `/Game/Radiation/BP_RadiationZone.MidRadiation` 0.0 _raditaionzoneref)
  (set `/Game/Radiation/BP_RadiationZone.HighRadiation` 0.05 _raditaionzoneref))

(fn `UserConstructionScript`
  (`parent.UserConstructionScript`))