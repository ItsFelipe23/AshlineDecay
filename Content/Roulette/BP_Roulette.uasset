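; Roulette wheel actor that spins a physics ball and announces the winning colour.
; Spin teleports the ball to its start position, applies a random Y impulse, flags spinning and starts a five-second timer.
; When it expires, a tiny sphere trace at the ball finds the component it rests on, including the wheel's own.
; That component's Black, Red or Green tag sets the index broadcast through ColourWon.
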(event `Spin`
  (`SceneComponent.K2_SetWorldLocation` (`self.Ball`) (`SceneComponent.K2_GetComponentLocation` (`self.BallStartPos`)) false false)
  (`PrimitiveComponent.AddImpulse` (`self.Ball`) (`KismetMathLibrary.MakeVector` 0.0 (`KismetMathLibrary.RandomFloatInRange` 9000.0 5000000.0)) "None" true)
  (set `self.IsSpinning` true)
  (`KismetSystemLibrary.K2_SetTimerDelegate` (delegate `DecideWinner`) 5.0))

(event `DecideWinner`
  (bind _returnvalue (`SceneComponent.K2_GetComponentLocation` (`self.Ball`)))
  (bind (_outhit _returnvalue_2) (`KismetSystemLibrary.SphereTraceSingleForObjects` :`Start` _returnvalue :`End` _returnvalue :`Radius` 1.0 :`ObjectTypes` (`|MakeArray` "ObjectTypeQuery15" :!type "EObjectTypeQuery Enum") :`bIgnoreSelf` false))
  (if _returnvalue_2
    (for _array_element (`ActorComponent.ComponentTags` (`.HitComponent` (`GameplayStatics.BreakHitResult` _outhit)))
      (switch `name` _array_element
        (:`Black`
          (`self.ColourWon` 0))
        (:`Red`
          (`self.ColourWon` 1))
        (:`Green`
          (`self.ColourWon` 2))))))

(fn `UserConstructionScript`)