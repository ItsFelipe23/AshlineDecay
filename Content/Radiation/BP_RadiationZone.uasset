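; BP_RadiationZone is a radiation hazard actor that changes the player's radiation according to depth within three nested spheres.
; Overlap begin and end events on players tagged "Player" choose the low, mid or high rate for the current sphere.
; A looping one-second timer passes that rate to the first-person character's Radiation function.
; Leaving the outer sphere restarts the timer with the reduction amount.
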(event `self.ReceiveBeginPlay`
  (bind _returnvalue (`GameplayStatics.GetActorOfClass` "/Game/FirstPerson/Blueprints/BP_BaseFirstPersonCharacter.BP_BaseFirstPersonCharacter_C"))
  (set `self.PlayerCharacterREF` _returnvalue))

(event `self.LeastRadSphere.OnComponentBeginOverlap`
  (params (OverlappedComponent :type "PrimitiveComponent Object Reference") (OtherActor :type "Actor Object Reference") (OtherComp :type "PrimitiveComponent Object Reference") (OtherBodyIndex :type Integer) (bFromSweep :type Boolean) (SweepResult :type "HitResult Structure (by ref)"))
  (if (`self.ActorHasTag` OtherActor "Player")
    (`self.StartRadiation` (`self.LowRadiation`))))

(event `self.CloseRadSpher.OnComponentEndOverlap`
  (params (OverlappedComponent :type "PrimitiveComponent Object Reference") (OtherActor :type "Actor Object Reference") (OtherComp :type "PrimitiveComponent Object Reference") (OtherBodyIndex :type Integer))
  (if (`self.ActorHasTag` OtherActor "Player")
    (`self.StartRadiation` (`self.MidRadiation`))))

(event `self.MidRadSphere.OnComponentBeginOverlap`
  (params (OverlappedComponent :type "PrimitiveComponent Object Reference") (OtherActor :type "Actor Object Reference") (OtherComp :type "PrimitiveComponent Object Reference") (OtherBodyIndex :type Integer) (bFromSweep :type Boolean) (SweepResult :type "HitResult Structure (by ref)"))
  (if (`self.ActorHasTag` OtherActor "Player")
    (`self.StartRadiation` (`self.MidRadiation`))))

(event `self.MidRadSphere.OnComponentEndOverlap`
  (params (OverlappedComponent :type "PrimitiveComponent Object Reference") (OtherActor :type "Actor Object Reference") (OtherComp :type "PrimitiveComponent Object Reference") (OtherBodyIndex :type Integer))
  (if (`self.ActorHasTag` OtherActor "Player")
    (`self.StartRadiation` (`self.LowRadiation`))))

(event `self.CloseRadSpher.OnComponentBeginOverlap`
  (params (OverlappedComponent :type "PrimitiveComponent Object Reference") (OtherActor :type "Actor Object Reference") (OtherComp :type "PrimitiveComponent Object Reference") (OtherBodyIndex :type Integer) (bFromSweep :type Boolean) (SweepResult :type "HitResult Structure (by ref)"))
  (if (`self.ActorHasTag` OtherActor "Player")
    (`self.StartRadiation` (`self.HighRadiation`))))

(event `self.LeastRadSphere.OnComponentEndOverlap`
  (params (OverlappedComponent :type "PrimitiveComponent Object Reference") (OtherActor :type "Actor Object Reference") (OtherComp :type "PrimitiveComponent Object Reference") (OtherBodyIndex :type Integer))
  (if (`self.ActorHasTag` OtherActor "Player")
    (`KismetSystemLibrary.K2_ClearAndInvalidateTimerHandle` (`self.RadiationTimerHandle`))
    (`self.StartRadiation` (`self.ReduceRadiationAmount`))))

(event `StartRadiation`
  (params (RadiationToApply :type "Float (double-precision)"))
  (bind _returnvalue (`KismetSystemLibrary.K2_SetTimerDelegate` (delegate `ApplyRadiation`) 1.0 true))
  (set `self.RadiationTimerHandle` _returnvalue))

(event `ApplyRadiation`
  (`/Game/FirstPerson/Blueprints/BP_BaseFirstPersonCharacter.Radiation` (`self.PlayerCharacterREF`) (stale `StartRadiation` RadiationToApply)))

(fn `UserConstructionScript`)