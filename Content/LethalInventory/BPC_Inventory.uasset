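; Inventory component for a four-slot hotbar that stores item names and mirrors them to an inventory bar widget.
; Number keys and the mouse wheel move the highlighted slot, with the wheel wrapping around.
; Pickups fill only the current slot if it is free, and clearing empties that slot.
; A saved pistol slot index drives IsHoldingWeapon, rechecked on number keys but on wheel scrolls only when wrapping.
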(event `ClearItemSlot`
  (if (not (== (`|GetArrayItem` (`self.InventorySlots`) (`self.CurrentSlotIndex`)) "None"))
    (`self.ClearSlot`)))

(event `Initialise`
  (params (InventoryBarREF :type "/Game/LethalInventory/Widgets/WBP_InventoryBar Object Reference"))
  (set `self.InventoryBar` InventoryBarREF)
  (`/Game/LethalInventory/Widgets/WBP_InventoryBar.HighlightSlot` (`self.InventoryBar`) 0))

(event `Key|MouseScrollUp`
  (params (Key :type "Key Structure"))
  (:`Pressed`
    (`/Game/LethalInventory/Widgets/WBP_InventoryBar.UnhighlightSlot` (`self.InventoryBar`) (`self.CurrentSlotIndex`))
    (bind _output_get (set `self.CurrentSlotIndex` (+ (`self.CurrentSlotIndex`) 1)))
    (if (>= _output_get 4)
      (bind _output_get_2 (set `self.CurrentSlotIndex` 0))
      (`/Game/LethalInventory/Widgets/WBP_InventoryBar.HighlightSlot` (`self.InventoryBar`) _output_get_2)
      (`self.CheckForPistol` _output_get_2)
      (else
        (`/Game/LethalInventory/Widgets/WBP_InventoryBar.HighlightSlot` (`self.InventoryBar`) (`self.CurrentSlotIndex`))))))

(event `Key|One`
  (params (Key :type "Key Structure"))
  (:`Pressed`
    (`/Game/LethalInventory/Widgets/WBP_InventoryBar.UnhighlightSlot` (`self.InventoryBar`) (`self.CurrentSlotIndex`))
    (bind _output_get (set `self.CurrentSlotIndex` 0))
    (`/Game/LethalInventory/Widgets/WBP_InventoryBar.HighlightSlot` (`self.InventoryBar`) _output_get)
    (`self.CheckForPistol` _output_get)))

(event `Key|Two`
  (params (Key :type "Key Structure"))
  (:`Pressed`
    (`/Game/LethalInventory/Widgets/WBP_InventoryBar.UnhighlightSlot` (`self.InventoryBar`) (`self.CurrentSlotIndex`))
    (bind _output_get (set `self.CurrentSlotIndex` 1))
    (`/Game/LethalInventory/Widgets/WBP_InventoryBar.HighlightSlot` (`self.InventoryBar`) _output_get)
    (`self.CheckForPistol` _output_get)))

(event `Key|Three`
  (params (Key :type "Key Structure"))
  (:`Pressed`
    (`/Game/LethalInventory/Widgets/WBP_InventoryBar.UnhighlightSlot` (`self.InventoryBar`) (`self.CurrentSlotIndex`))
    (bind _output_get (set `self.CurrentSlotIndex` 2))
    (`/Game/LethalInventory/Widgets/WBP_InventoryBar.HighlightSlot` (`self.InventoryBar`) _output_get)
    (`self.CheckForPistol` _output_get)))

(event `Key|MouseScrollDown`
  (params (Key :type "Key Structure"))
  (:`Pressed`
    (`/Game/LethalInventory/Widgets/WBP_InventoryBar.UnhighlightSlot` (`self.InventoryBar`) (`self.CurrentSlotIndex`))
    (bind _output_get (set `self.CurrentSlotIndex` (- (`self.CurrentSlotIndex`) 1)))
    (if (<= _output_get -1)
      (bind _output_get_2 (set `self.CurrentSlotIndex` 3))
      (`/Game/LethalInventory/Widgets/WBP_InventoryBar.HighlightSlot` (`self.InventoryBar`) _output_get_2)
      (`self.CheckForPistol` _output_get_2)
      (else
        (`/Game/LethalInventory/Widgets/WBP_InventoryBar.HighlightSlot` (`self.InventoryBar`) (`self.CurrentSlotIndex`))))))

(event `Key|Four`
  (params (Key :type "Key Structure"))
  (:`Pressed`
    (`/Game/LethalInventory/Widgets/WBP_InventoryBar.UnhighlightSlot` (`self.InventoryBar`) (`self.CurrentSlotIndex`))
    (bind _output_get (set `self.CurrentSlotIndex` 3))
    (`/Game/LethalInventory/Widgets/WBP_InventoryBar.HighlightSlot` (`self.InventoryBar`) _output_get)
    (`self.CheckForPistol` _output_get)))

(fn `CheckForPistol`
  (params (CurrentIndex :type Integer))
  (if (== CurrentIndex (`self.PistolIndex`))
    (set `self.isHoldingWeapon` true)
    (`KismetSystemLibrary.PrintString` "Pisotl")
    (else
      (set `self.isHoldingWeapon` false))))

(fn `ClearSlot`
  (`KismetArrayLibrary.Array_Set` (`self.InventorySlots`) (`self.CurrentSlotIndex`))
  (`/Game/LethalInventory/Widgets/WBP_InventoryBar.SlotChanged` (`self.InventoryBar`) (`self.CurrentSlotIndex`) null true))

(fn `GetItemInfo`
  (params (`Item Name` :type Name) (`Empty Element` :type Integer) (ItemImage :type "Texture2D Object Reference"))
  (if (== `Item Name` "Pistol")
    (set `self.PistolIndex` (`local.Empty Element`))
    (set `self.isHoldingWeapon` true))
  (`KismetArrayLibrary.Array_Set` (`self.InventorySlots`) (`local.Empty Element`) `Item Name`)
  (`/Game/LethalInventory/Widgets/WBP_InventoryBar.SlotChanged` (`self.InventoryBar`) (`local.Empty Element`) ItemImage false))

(fn `IsSlotFree?`
  (params (`Object Name` :type Name) (ItemImage :type "Texture2D Object Reference"))
  (returns (EmptySlot :type Boolean))
  (if (== (`|GetArrayItem` (`self.InventorySlots`) (`self.CurrentSlotIndex`)) "None")
    (`self.GetItemInfo` `Object Name` (`self.CurrentSlotIndex`) ItemImage)
    (return true)
    (else
      (return false))))