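; BP_Scanner is a scan pulse actor that expands a sphere outward and highlights the actors it touches.
; DoScan stores the MutatedScan value, enables query collision, then plays a timeline driving actor scale and the sphere material's ScannerOpacity.
; Each actor that begins overlapping receives HighlightScanMessage with that stored value.
; When the timeline finishes, the scanner disables collision, collapses to zero scale and hides itself.
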(event `DoScan`
  (params (MutatedScan :type Boolean))
  (set `self.MutatedScan` MutatedScan)
  (`PrimitiveComponent.SetCollisionEnabled` (`self.Sphere`) "QueryOnly")
  (`self.SetActorHiddenInGame` false)
  (bind (_direction _scannerexpandsize _scanneropacity) (`Timeline|ExpandScanner`)
    (:`Update`
      (`self.SetActorScale3D` (`KismetMathLibrary.Conv_DoubleToVector` _scannerexpandsize))
      (`MeshComponent.SetScalarParameterValueOnMaterials` (`self.Sphere`) "ScannerOpacity" _scanneropacity))
    (:`Finished`
      (`PrimitiveComponent.SetCollisionEnabled` (`self.Sphere`) "NoCollision")
      (`self.SetActorScale3D` (0.0 0.0 0.0))
      (`self.SetActorHiddenInGame` true))))

(event `self.Sphere.OnComponentBeginOverlap`
  (params (OverlappedComponent :type "PrimitiveComponent Object Reference") (OtherActor :type "Actor Object Reference") (OtherComp :type "PrimitiveComponent Object Reference") (OtherBodyIndex :type Integer) (bFromSweep :type Boolean) (SweepResult :type "HitResult Structure (by ref)"))
  (message `/Game/FirstPerson/Blueprints/Interfaces/BPI_Masters.HighlightScan` OtherActor (`self.MutatedScan`)))

(fn `UserConstructionScript`)