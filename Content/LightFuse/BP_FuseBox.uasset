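; BP_FuseBox is an interactable fuse box that checks whether the player holds the piece that fits it.
; Interact stores the interacting player and reads the picked-up item from their player struct, testing it for the "Switch" actor tag.
; A missing or wrong item updates the player's prompt with a hint, while a matching one only prints a debug string.
; SpawnPurchasedItem is an unimplemented stub returning false.
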(event `/Game/FirstPerson/Blueprints/Interfaces/BPI_Masters.Interact`
  (params (InteractingPlayer :type "/Game/FirstPerson/Blueprints/PlayerCharacter/BP_BaseFirstPersonCharacter Object Reference"))
  (bind ((`PickedUpItem_81_ED25D74A4E9209BA9440D7BDF47D96B8` _pickedupitem)) (break `/Game/FirstPerson/Blueprints/Structs/S_PlayerStruct` (`/Game/FirstPerson/Blueprints/PlayerCharacter/BP_BaseFirstPersonCharacter.S_PlayerStruct` InteractingPlayer)))
  (set `self.Interacting Player` InteractingPlayer)
  (`/Engine/EditorBlueprintResources/StandardMacros.IsValid` _pickedupitem
    (:`Is Valid`
      (if (`self.ActorHasTag` _pickedupitem "Switch")
        (`KismetSystemLibrary.PrintString` "Hello")
        (else
          (`/Game/FirstPerson/Blueprints/PlayerCharacter/BP_BaseFirstPersonCharacter.E_UpdatePrompt` (`self.Interacting Player`) "This looks like the wrong piece..."))))
    (:`Is Not Valid`
      (`/Game/FirstPerson/Blueprints/PlayerCharacter/BP_BaseFirstPersonCharacter.E_UpdatePrompt` (`self.Interacting Player`) "Something fits here..."))))

(fn `SpawnPurchasedItem`
  (params (ItemToSpawn :type "/Game/Perks/BP_BaseConsumable Class Reference"))
  (returns (CanSpawn :type Boolean))
  (return false))

(fn `UserConstructionScript`)