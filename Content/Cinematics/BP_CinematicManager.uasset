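; BP_CinematicManager plays the opening and closing door cinematics when the room generator requests them.
; On BeginPlay it binds to the EPlayCinematic dispatcher on RoomGenREF.
; PlayCinematic switches on the requested cinematic type and routes to a handler that passes a fixed index to PlayChosenCinematic.
; That function plays the SequencePlayer of the matching CinematicsToPlay entry, so array order must match the cinematic types.
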(event `self.ReceiveBeginPlay`
  (add `/Game/ProceduralRooms/BP_RoomGeneratorManager.E_PlayCinematic` (`self.RoomGenREF`) (`|CreateDelegate` :!event `PlayCinematic`)))

(event `PlayCinematic`
  (params (CinematicToPlay :type "/Game/Cinematics/E_CinematicToPlay Enum" :default "NewEnumerator0"))
  (switch `/Game/Cinematics/E_CinematicToPlay` CinematicToPlay
    (:`NewEnumerator0`
      (`self.PlayBeginningCinematic`))
    (:`NewEnumerator1`
      (`self.ClosingDoorsCinematic`))))

(event `PlayBeginningCinematic`
  (`self.PlayChosenCinematic` 0))

(event `ClosingDoorsCinematic`
  (`self.PlayChosenCinematic` 1))

(fn `PlayChosenCinematic`
  (params (CinematicIndex :type Integer))
  (`MovieSceneSequencePlayer.Play` (`LevelSequenceActor.SequencePlayer` (`|GetArrayItem` (`self.CinematicsToPlay`) CinematicIndex))))

(fn `UserConstructionScript`)